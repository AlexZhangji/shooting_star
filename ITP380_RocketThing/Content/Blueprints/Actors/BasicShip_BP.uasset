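; BasicShip_BP is a player ship with homing missiles, a shield and a rewind ability, colored by player number.
; HomingMissle input fires a timed five-missile volley, and Interceptor switches that player's live missiles to attack mode via an owner ID search.
; Tick applies ShieldIsOn to the sphere's mesh, and DeactivateShield turns it off with a sound.
; Rewind input conditionally spawns a player-tagged RewindActor at the ship's location.
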(event EventBeginPlay
  (Utilities|FlowControl|Delay 0.2)
  (Variables|Default|SetAB1 (Utilities|Array|Get(acopy) (Variables|Default|GetAbilityList)))
  ;[1 1 1] sphere invisable
  (Components|StaticMesh|SetStaticMesh (Variables|Default|GetSphere) 0)
  (Utilities|FlowControl|Delay 1.0)
  ;[1 1 1] create point light
  (CallFunction|InitRandomColor)
  (Rendering|Components|Light|SetLightColor (Variables|Default|GetPointLight) (Utilities|Array|Get(acopy) (Variables|Default|GetShipLightList) (Variables|Default|GetPlayerNumber)))
  (Utilities|Casting|CastToBasicShip_BP self
    (:CastFailed
      (Development|PrintString "failed cast ship"))))

(event EventActorBeginOverlap
  (params (OtherActor :type Actor%20Object%20Reference)))

(event EventTick
  (params (DeltaSeconds :type Float%20%28single-precision%29))
  ;[1 1 1] This was when I have no idea i can use branch in BP...
  (switch int (Variables|Default|GetShieldIsOn)
    (:0
      (CallFunction|DisableShield))
    (:1
      (CallFunction|EnableShield))))

(event Input|ActionEvents|InputActionRewind
  (bind _self self)
  (:Pressed
    (Utilities|FlowControl|Delay 0.2)
    (if (and (Variables|/Script/ITP380_RocketThing.Ship|GetbRewindInProcess _self) (Variables|/Script/ITP380_RocketThing.Ship|GetbCanSpawnIlussion _self))
      (bind _returnvalue (Game|SpawnActorfromClass "/Game/Blueprints/Actors/rewindActor.rewindActor_C" (Math|Conversions|ToTransform(Vector) (Transformation|GetActorLocation)) false 0))
      (Variables|/Game/Blueprints/Actors/rewindActor.rewindActor_C|SetrewinActorNum _returnvalue (Variables|Default|GetPlayerNum))
      (Variables|/Script/ITP380_RocketThing.Ship|SetbCanSpawnIlussion self false))))

(event Input|ActionEvents|InputActionHomingMissle
  (:Pressed
    (if (not (Variables|/Script/ITP380_RocketThing.Ship|GetbHomingInProcess self))
      (Utilities|FlowControl|Delay 0.4)
      (if (Variables|/Script/ITP380_RocketThing.Ship|GetbCDHoming self)
        (Class|GameplayStatics|PlaySoundAttached "/Game/Sound/HomingStart_Cue.HomingStart_Cue" (Variables|Default|GetShipMeshComponent))
        (Utilities|Spawn5withDelay)))))

(event Input|ActionEvents|InputActionDeactivateShield
  (:Pressed
    (switch int (Variables|Default|GetShieldIsOn)
      (:1
        (CallFunction|DisableShield)
        (Class|GameplayStatics|PlaySoundAttached "/Game/Sound/deactive_Cue.deactive_Cue" (Variables|Default|GetShipMeshComponent))))))

(event Input|ActionEvents|InputActionInterceptor
  (:Pressed
    (CallFunction|AttackModeonforHomingMissle)))

(fn ConstructionScript)

(fn GetHealthRatio
  (bind _self self)
  (return (Math|Float|Clamp(Float) (/ (Variables|/Script/ITP380_RocketThing.Ship|Gethealth _self) (Variables|/Script/ITP380_RocketThing.Ship|GetMaxHealth _self)))))

(fn InitRandomColor
  (switch int (Variables|Default|GetPlayerNumber)
    (:1
      (Variables|Default|SetShipColor (Variables|Default|GetcolorInstance1)))
    (:2
      (Variables|Default|SetShipColor (Variables|Default|GetcolorInstance2))))
  (return ""))

(fn EnableShield
  (bind _sphere (Variables|Default|GetSphere))
  (Variables|Default|SetShieldIsOn 1)
  (Components|StaticMesh|SetStaticMesh _sphere "/Game/TwinStick/Meshes/protectiveShiledMesh.protectiveShiledMesh")
  (Rendering|Material|SetMaterial _sphere 0 "/Game/Assets/Materials/transBlue.transBlue"))

(fn DisableShield
  (Components|StaticMesh|SetStaticMesh (Variables|Default|GetSphere) 0)
  (Variables|Default|SetShieldIsOn 0))

(fn SpawnMissle
  (bind _self self)
  (bind _returnvalue (Game|SpawnActorfromClass "/Game/Blueprints/Actors/HMissile.HMissile_C" (Math|Transform|MakeTransform (Transformation|GetActorLocation _self) (Transformation|GetActorRotation _self) "2.000000,0.700000,1.300000") false 0))
  (Default|InitHoming _returnvalue self (Variables|Default|GetPlayerNum)))

(fn AttackModeonforHomingMissle
  (if (Variables|/Script/ITP380_RocketThing.Ship|GetbCDHoming self)
    (if (not (Variables|Default|GetHomingAttackMode))
      (Class|GameplayStatics|PlaySoundAttached "/Game/Sound/AttackMode_Cue.AttackMode_Cue" (Variables|Default|GetShipMeshComponent))
      (bind _outactors (Actor|GetAllActorsOfClass "/Game/Blueprints/Actors/HMissile.HMissile_C"))
      (for _index (range 0 (Utilities|Array|Length _outactors))
        (if (== (Variables|/Game/Blueprints/Actors/HMissile.HMissile_C|GetOwnerID (Utilities|Array|Get(acopy) _outactors _index)) (Variables|Default|GetPlayerNum))
          (Default|AttackModeon (Utilities|Array|Get(acopy) _outactors _index))
          (Variables|Default|SetHomingAttackMode true))))))

(fn InitWeaponColor)

(fn InitWeaponNum
  (for _index (range 0 (Utilities|Array|Length (Variables|/Script/ITP380_RocketThing.Ship|GetWeapons self)))
    _))