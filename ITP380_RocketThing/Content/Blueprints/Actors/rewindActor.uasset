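; Short-lived helper actor tied to one BasicShip_BP, watching for that ship's rewind to end.
; Tick runs through a 0.3-second Delay, then fetches all ships and picks one by the RewinActorNum index.
; While that ship's RewindInProcess is true, it effectively does nothing.
; Otherwise it sets the ship's CanSpawnIlussion flag and destroys itself.
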(event EventBeginPlay)

(event EventActorBeginOverlap
  (params (OtherActor :type Actor%20Object%20Reference)))

(event EventTick
  (params (DeltaSeconds :type Float%20%28single-precision%29))
  (Utilities|FlowControl|Delay 0.3)
  (bind _outactors (Actor|GetAllActorsOfClass "/Game/Blueprints/Actors/BasicShip_BP.BasicShip_BP_C"))
  (if (Variables|/Script/ITP380_RocketThing.Ship|GetbRewindInProcess (Utilities|Array|Get(acopy) _outactors (Variables|Default|GetrewinActorNum)))
    (Variables|Default|SetrewinActorNum (Variables|Default|GetrewinActorNum))
    (else
      (Variables|/Script/ITP380_RocketThing.Ship|SetbCanSpawnIlussion (Utilities|Array|Get(acopy) _outactors (Variables|Default|GetrewinActorNum)) true)
      (Actor|DestroyActor self))))

(fn ConstructionScript)

(fn NewFunction0)