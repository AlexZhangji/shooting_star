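; Homing missile for multiplayer ship combat, coloured by owner, that homes on its owner's ship until switched to attack mode.
; AttackModeOn retargets it to the opponent in two-player games or the ship nearest the owner otherwise, and lowers its speed limits.
; One second after overlapping a non-owner ship, it damages the stored target player's pawn and explodes.
; A lifetime timer destroys it, clearing the owner's attack flag.
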(event OnComponentBeginOverlap(FirableMesh)
  (params (OtherActor :type Actor%20Object%20Reference) (OtherComp :type Primitive%20Component%20Object%20Reference) (OtherBodyIndex :type Integer) (bFromSweep :type Boolean) (SweepResult :type Hit%20Result%20Structure%20%28by%20ref%29))
  (bind _asbasic_ship_bp (Utilities|Casting|CastToBasicShip_BP OtherActor))
  (Utilities|FlowControl|Delay 1.0)
  (bind _outactors (Actor|GetAllActorsOfClass "/Game/Blueprints/Actors/BasicShip_BP.BasicShip_BP_C"))
  (if (not (== _asbasic_ship_bp (Utilities|Array|Get(acopy) _outactors (Variables|Default|GetOwnerID))))
    (for _index (range 0 (Variables|/Game/Blueprints/Actors/BasicShip_BP.BasicShip_BP_C|GettotalNum (Utilities|Array|Get(acopy) _outactors)))
      (if (not (== _index (Variables|Default|GetOwnerID)))
        (CallFunction|ApplyDamageHelper _index)))))

(event EventBeginPlay)

(event EventTick
  (params (DeltaSeconds :type Float%20%28single-precision%29)))

(fn ConstructionScript)

(fn InitHoming
  (params (ship :type Basic%20Ship%20BP%20Object%20Reference) (OwnerID_int :type Integer :default 0))
  (bind _self self)
  (bind _projectilemovement (Variables|Default|GetProjectileMovement))
  ;[1 1 1] dynamicly assign color to mesh
  (Variables|Default|SetOwnerID OwnerID_int)
  (Rendering|Material|SetMaterial (Variables|Default|GetFirableMesh) 0 (Utilities|Array|Get(acopy) (Variables|/Game/Blueprints/Actors/BasicShip_BP.BasicShip_BP_C|GetMaterialList ship) OwnerID_int))
  (Utilities|Time|SetTimerbyFunctionName _self "selfDestroy" (Math|Conversions|ToFloat(Integer) (Variables|Default|GetlastingTime)))
  (Variables|Default|SetDamageHoming (Variables|/Script/ITP380_RocketThing.Firable|GetDamage _self))
  (bind _outactors (Actor|GetAllActorsOfClass "/Game/Blueprints/Actors/BasicShip_BP.BasicShip_BP_C"))
  (if (== (Variables|/Game/Blueprints/Actors/BasicShip_BP.BasicShip_BP_C|GettotalNum (Utilities|Array|Get(acopy) _outactors)) 1)
    ;[1 1 1] get oppoent instance
    (bind _outactors_2 (Actor|GetAllActorsOfClass "/Game/Blueprints/Actors/BasicShip_BP.BasicShip_BP_C"))
    (if (== (Variables|Default|GetOwnerID) 0)
      (Variables|/Script/Engine.ProjectileMovementComponent|SetHomingTargetComponent _projectilemovement (Variables|/Script/ITP380_RocketThing.Ship|GetShipMeshComponent (Utilities|Array|Get(acopy) _outactors_2)))
      (Variables|Default|SetP1 (Utilities|Array|Get(acopy) _outactors_2 1))
      (else
        (Variables|/Script/Engine.ProjectileMovementComponent|SetHomingTargetComponent _projectilemovement (Variables|/Script/ITP380_RocketThing.Ship|GetShipMeshComponent (Utilities|Array|Get(acopy) _outactors_2 1)))
        (Variables|Default|SetP1 (Utilities|Array|Get(acopy) _outactors_2))))
    (Variables|Default|SetOwnerInstance (Utilities|Array|Get(acopy) _outactors_2 (Variables|Default|GetOwnerID)))
    (Variables|Default|SethomingID 0)
    (else
      (Variables|/Script/Engine.ProjectileMovementComponent|SetHomingTargetComponent (Variables|Default|GetProjectileMovement) (Variables|/Script/ITP380_RocketThing.Ship|GetShipMeshComponent (Utilities|Array|Get(acopy) _outactors (Variables|Default|GetOwnerID)))))))

(fn SelfDestroy
  (bind _self self)
  (bind _ownerinstance (Variables|Default|GetOwnerInstance))
  (if (Variables|Default|GetAttackMode)
    (Effects|SpawnEmitteratLocation (Variables|Default|Getfx) (Transformation|GetActorLocation _self))
    (Variables|/Game/Blueprints/Actors/BasicShip_BP.BasicShip_BP_C|SetHomingAttackMode _ownerinstance false)
    (else
      (Variables|/Game/Blueprints/Actors/BasicShip_BP.BasicShip_BP_C|SetHomingAttackMode _ownerinstance false)))
  (Actor|DestroyActor _self))

(fn SlowSpeed
  (bind _projectilemovement (Variables|Default|GetProjectileMovement))
  (Variables|/Script/Engine.ProjectileMovementComponent|SetInitialSpeed _projectilemovement 5e+02)
  (Variables|/Script/Engine.ProjectileMovementComponent|SetMaxSpeed _projectilemovement 6e+02))

(fn AttackModeon
  (if (Variables|Default|GetAttackMode)
    _
    (else
      _))
  (Variables|Default|SetAttackMode true)
  (bind _outactors (Actor|GetAllActorsOfClass "/Game/Blueprints/Actors/BasicShip_BP.BasicShip_BP_C"))
  (if (== (Variables|/Game/Blueprints/Actors/BasicShip_BP.BasicShip_BP_C|GettotalNum (Utilities|Array|Get(acopy) _outactors)) 1)
    (Variables|/Script/Engine.ProjectileMovementComponent|SetHomingTargetComponent (Variables|Default|GetProjectileMovement) (Variables|/Script/ITP380_RocketThing.Ship|GetShipMeshComponent (Variables|Default|GetP1)))
    (if (== (Variables|Default|GetOwnerID) 0)
      (Variables|Default|SethomingID 1)
      (else
        (Variables|Default|SethomingID 0)))
    (else
      (CallFunction|GetClosestShip (Variables|Default|GetOwnerID))))
  (CallFunction|SlowSpeed))

(fn GetClosestShip
  (params (OwnerID :type Integer :default 0))
  (bind _outactors (Actor|GetAllActorsOfClass "/Game/Blueprints/Actors/BasicShip_BP.BasicShip_BP_C"))
  (Variables|Default|SetOwnerInstance (Utilities|Array|Get(acopy) _outactors OwnerID))
  (for _index (range 0 3)
    (if (not (== _index OwnerID))
      (CallFunction|GetCloseHelper _index)))
  (Variables|/Script/Engine.ProjectileMovementComponent|SetHomingTargetComponent (Variables|Default|GetProjectileMovement) (Variables|/Script/ITP380_RocketThing.Ship|GetShipMeshComponent (Variables|Default|GetP1))))

(fn GetCloseHelper
  (params (num :type Integer :default 0))
  (bind _outactors (Actor|GetAllActorsOfClass "/Game/Blueprints/Actors/BasicShip_BP.BasicShip_BP_C"))
  (Math|Float|CompareFloat (Transformation|GetDistanceTo (Utilities|Array|Get(acopy) _outactors num) (Variables|Default|GetOwnerInstance)) (Variables|Default|GetDistanceToActor)
    (:<
      (Variables|Default|SetDistanceToActor (Transformation|GetDistanceTo (Utilities|Array|Get(acopy) _outactors num) (Variables|Default|GetOwnerInstance)))
      (Variables|Default|SetP1 (Utilities|Array|Get(acopy) _outactors num))
      (Variables|Default|SethomingID num))))

(fn ApplyDamageHelper
  (params (NewParam :type Integer :default 0))
  (bind _self self)
  (if (== (Variables|Default|GethomingID) NewParam)
    (Game|Damage|ApplyDamage (Game|Player|GetPlayerPawn NewParam) (Variables|Default|GetDamageHoming) (Game|GetPlayerController NewParam) (Game|GetInstigator self) "/Script/Engine.DamageType")
    (Effects|SpawnEmitteratLocation (Variables|Default|Getfx) (Transformation|GetActorLocation _self) "0.000000, 0, 0")
    (Actor|DestroyActor _self)))