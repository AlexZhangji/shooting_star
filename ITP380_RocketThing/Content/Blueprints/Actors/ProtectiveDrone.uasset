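; Homing drone spawned for one of two ships, which chases the opposing ship and damages any actor it hits until it expires.
; A one-shot on the first Tick runs InitHoming, coloring the mesh from the owner's material list, copying damage and starting the self-destruct timer.
; InitHoming also picks the homing target by indexing the ship array with OwnerID.
; Hits leave the drone alive, as its effect-and-destroy branch is disconnected.
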(event EventBeginPlay)

(event EventTick
  (params (DeltaSeconds :type Float%20%28single-precision%29))
  (Utilities|FlowControl|DoOnce false
    (:Completed
      (CallFunction|InitHoming))))

(event EventHit
  (params (MyComp :type Primitive%20Component%20Object%20Reference) (Other :type Actor%20Object%20Reference) (OtherComp :type Primitive%20Component%20Object%20Reference) (bSelfMoved :type Boolean) (HitLocation :type Vector :default "0, 0, 0") (HitNormal :type Vector :default "0, 0, 0") (NormalImpulse :type Vector :default "0, 0, 0") (Hit :type Hit%20Result%20Structure%20%28by%20ref%29))
  (Game|Damage|ApplyDamage Other (Variables|Default|GetDamageHoming) 0 self))

(fn ConstructionScript)

(fn InitHoming
  (bind _self self)
  (bind _projectilemovement (Variables|Default|GetProjectileMovement))
  (bind _ownerid (Variables|Default|GetOwnerID))
  ;[1 1 1] dynamicly assign color to mesh
  (bind _outactors (Actor|GetAllActorsOfClass "/Game/Blueprints/Actors/BasicShip_BP.BasicShip_BP_C"))
  (Rendering|Material|SetMaterial (Variables|Default|GetFirableMesh) 0 (Utilities|Array|Get(acopy) (Variables|/Game/Blueprints/Actors/BasicShip_BP.BasicShip_BP_C|GetMaterialList (Utilities|Array|Get(acopy) _outactors _ownerid)) _ownerid))
  (Utilities|Time|SetTimerbyFunctionName _self "selfDestroy" (Math|Conversions|ToFloat(Integer) (Variables|Default|GetlastingTime)))
  (Variables|Default|SetDamageHoming (Variables|/Script/ITP380_RocketThing.Firable|GetDamage _self))
  ;[1 1 1] get oppoent instance
  (bind _outactors_2 (Actor|GetAllActorsOfClass "/Game/Blueprints/Actors/BasicShip_BP.BasicShip_BP_C"))
  (if (== (Variables|Default|GetOwnerID) 0)
    (Variables|/Script/Engine.ProjectileMovementComponent|SetHomingTargetComponent _projectilemovement (Variables|/Script/ITP380_RocketThing.Ship|GetShipMeshComponent (Utilities|Array|Get(acopy) _outactors_2 1)))
    (else
      (Variables|/Script/Engine.ProjectileMovementComponent|SetHomingTargetComponent _projectilemovement (Variables|/Script/ITP380_RocketThing.Ship|GetShipMeshComponent (Utilities|Array|Get(acopy) _outactors_2))))))

(fn SelfDestroy
  (Actor|DestroyActor self))