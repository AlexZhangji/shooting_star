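; WeaponProjectile_BP is a weapon projectile that colors itself to match its owner.
; On Tick, until ColorValid is set, it calls CheckColor, which reads OwnerID-indexed material and hit-effect lists from the first BasicShip_BP found.
; If material display names differ at index OwnerID, it sets FirableMesh's slot 0 material and HitFX, then always marks the color valid.
; The Trail template assignment is disconnected and never runs.
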(event EventBeginPlay)

(event EventActorBeginOverlap
  (params (OtherActor :type Actor%20Object%20Reference)))

(event EventTick
  (params (DeltaSeconds :type Float%20%28single-precision%29))
  (if (not (Variables|Default|GetbColorValid))
    (CallFunction|CheckColor)))

(fn ConstructionScript)

(fn CheckColor
  (bind _self self)
  (bind _firablemesh (Variables|Default|GetFirableMesh))
  (bind _ownerid (Variables|/Script/ITP380_RocketThing.Firable|GetOwnerID _self))
  (bind _outactors (Actor|GetAllActorsOfClass "/Game/Blueprints/Actors/BasicShip_BP.BasicShip_BP_C"))
  (if (Utilities|Enum|Equal(Enum) (Utilities|GetDisplayName (Utilities|Array|Get(acopy) (Rendering|Material|GetMaterials _firablemesh) (Variables|/Script/ITP380_RocketThing.Firable|GetOwnerID self))) (Utilities|GetDisplayName (Utilities|Array|Get(acopy) (Variables|/Game/Blueprints/Actors/BasicShip_BP.BasicShip_BP_C|GetMaterialList (Utilities|Array|Get(acopy) _outactors)) _ownerid)))
    _
    (else
      (Rendering|Material|SetMaterial _firablemesh 0 (Utilities|Array|Get(acopy) (Variables|/Game/Blueprints/Actors/BasicShip_BP.BasicShip_BP_C|GetMaterialList (Utilities|Array|Get(acopy) _outactors)) _ownerid))
      (Variables|/Script/ITP380_RocketThing.Firable|SetHitFX self (Utilities|Array|Get(acopy) (Variables|/Game/Blueprints/Actors/BasicShip_BP.BasicShip_BP_C|GetFXList (Utilities|Array|Get(acopy) _outactors)) _ownerid))))
  (Variables|Default|SetbColorValid true))