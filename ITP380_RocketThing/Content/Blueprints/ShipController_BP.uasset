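; ShipController_BP is a controller that triggers the two abilities of the possessed BasicShip_BP.
; Each ability input casts the controlled pawn to the ship and calls its matching use-ability function.
; After a fixed seven-second delay, it disables the shield if that ability slot holds Shield, so shield timeout is handled in the controller.
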(event EventBeginPlay)

(event EventTick
  (params (DeltaSeconds :type Float%20%28single-precision%29)))

(event Input|ActionEvents|InputActionUseFirstAbility
  (:Pressed
    (bind _asbasic_ship_bp (Utilities|Casting|CastToBasicShip_BP (Pawn|GetControlledPawn)))
    (Default|UseFirstAbilityBP _asbasic_ship_bp)
    (Utilities|FlowControl|Delay 7.0)
    (if (Utilities|Enum|Equal(Enum) (Variables|/Script/ITP380_RocketThing.Ship|GetfirstAbility _asbasic_ship_bp) "Shield")
      (Default|DisableShield _asbasic_ship_bp))))

(event Input|ActionEvents|InputActionUseSecondAbility
  (:Pressed
    (bind _asbasic_ship_bp (Utilities|Casting|CastToBasicShip_BP (Pawn|GetControlledPawn)))
    (Default|UseSecondAbilityBP _asbasic_ship_bp)
    (Utilities|FlowControl|Delay 7.0)
    (if (Utilities|Enum|Equal(Enum) (Variables|/Script/ITP380_RocketThing.Ship|GetsecondAbility _asbasic_ship_bp) "Shield")
      (Default|DisableShield _asbasic_ship_bp))))

(fn ConstructionScript)